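; PlatLight is a configurable light actor with a SpotLight and a PointLight, set up once at BeginPlay.
; The IsClose flag hides the spot light and skips all further setup, leaving the point light's visibility untouched.
; Otherwise, variables drive the spot light's intensity, color, attenuation radius and cone angles, plus the point light's intensity, with its color forced to white.
; The construction script is empty, so these values apply only at runtime.
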(event EventBeginPlay
  (bind _isclose (Variables|Default|GetIsClose))
  (bind _spotlight (Variables|Default|GetSpotLight))
  (bind _pointlight (Variables|Default|GetPointLight))
  (bind _returnvalue (not _isclose))
  (Rendering|SetVisibility (Variables|Default|GetSpotLight) _returnvalue false)
  (if _returnvalue
    (Utilities|FlowControl|Sequence
      (:then_0
        (Rendering|Components|Light|SetIntensity _spotlight (Variables|Default|GetFireIntensity))
        (Rendering|Components|Light|SetLightColor _spotlight (Variables|Default|GetLightColor) true)
        (Rendering|Lighting|SetAttenuationRadius _spotlight (Variables|Default|GetDecayR))
        (Rendering|Lighting|SetInnerConeAngle _spotlight (Variables|Default|GetInR))
        (Rendering|Lighting|SetOuterConeAngle _spotlight (Variables|Default|GetOutR)))
      (:then_1
        (Rendering|Components|Light|SetIntensity _pointlight (Variables|Default|GetPointLightIntensity))
        (Rendering|Components|Light|SetLightColor _pointlight (Utilities|Struct|MakeLinearColor 1.0 1.0 1.0 1.0) true)))))

(event Collision|EventActorBeginOverlap
  (params (OtherActor :type Actor%20Object%20Reference)))

(event EventTick
  (params (DeltaSeconds :type Float%20%28single-precision%29)))

(fn ConstructionScript)