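; Door actor that swings open once the game mode flags the third door as open.
; BeginPlay casts the game mode to ThirdPersonGameMode and caches it.
; Tick polls its BThirdDoorOpen flag every frame and calls Open while it is true.
; Open snaps the door mesh to a fixed relative rotation, with no animation or closing logic.
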(event EventBeginPlay
  (bind _asthird_person_game_mode (Utilities|Casting|CastToThirdPersonGameMode (Game|GetGameMode)))
  (Variables|Default|SetAs%20Third%20Person%20Game%20Mode _asthird_person_game_mode))

(event Collision|EventActorBeginOverlap
  (params (OtherActor :type Actor%20Object%20Reference)))

(event EventTick
  (params (DeltaSeconds :type Float%20%28single-precision%29))
  (if (Variables|/Game/ThirdPersonBP/Blueprints/ThirdPersonGameMode.ThirdPersonGameMode_C|GetB_ThirdDoorOpen (Variables|Default|GetAs%20Third%20Person%20Game%20Mode))
    (CallFunction|Open)))

(fn ConstructionScript)

(fn Open
  (Transformation|SetRelativeRotation (Variables|Default|GetSM_Door) "0,90.000000, 0" false false))